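; Actor Blueprint for a skeletal mesh tube that drives a continuously circling effector location in its ABP_SimpleTube animation instance.
; Each tick it advances a yaw angle by a fixed step, so the speed depends on frame rate, and rotates a scaled actor right vector by it.
; The resulting offset is written without adding the actor's location; OriginalLocation is saved at BeginPlay but unused here.
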(event `self.ReceiveBeginPlay`
  (set `self.OriginalLocation` (`self.K2_GetActorLocation`)))

(event `self.ReceiveTick`
  (params (DeltaSeconds :type "Float (single-precision)"))
  ;[1 1 1] Rotate
  (bind _output_get (set `self.Angle` (+ (`self.Angle`) 2.0)))
  (bind _asabp_simple_tube (cast `/Game/SimpleTube/ABP_SimpleTube` (`SkeletalMeshComponent.GetAnimInstance` (`self.SkeletalMesh`))))
  (set `/Game/SimpleTube/ABP_SimpleTube.EffectorLocation` (`KismetMathLibrary.GreaterGreater_VectorRotator` (* (`self.GetActorRightVector`) 300.0) (`KismetMathLibrary.MakeRotator` 0.0 0.0 _output_get)) _asabp_simple_tube))

(fn `UserConstructionScript`)